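; Zombie enemy character that chases the player's mecha, attacks it up close and ragdolls on death.
; Tick drives AI MoveTo; within melee range it pauses movement, plays the attack through anim blueprint flags, then rechecks range before flagging player damage.
; Bullet hits reduce HP and briefly stagger it.
; Depleted HP or explosion hits trigger an impulse-driven physics ragdoll, remove the capsule and destroy it after a delay.
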(event `self.ReceiveTick`
  (params (DeltaSeconds :type "Float (single-precision)"))
  (bind _charactermovement (`self.CharacterMovement`))
  ;[1 1 1] chase the player
  (bind _asmecha_char_cam (cast `/Game/Blueprints/mecha_char+cam` (`GameplayStatics.GetPlayerPawn` 0) :!label _label))
  (`|AIMoveTo` self (0.0 0.0 0.0) _asmecha_char_cam 20.0
    (:`then`
      (bind _returnvalue (and (not (`self.ided`)) (<= (`KismetMathLibrary.GetPointDistanceToLine` (`self.K2_GetActorLocation` _asmecha_char_cam) (`self.K2_GetActorLocation`)) 150.0)))
      (if _returnvalue
        (bind _aszombie_anim (cast `/Game/Blueprints/zombie_anim` (`SkeletalMeshComponent.GetAnimInstance` (`self.Mesh`))))
        (set `/Game/Blueprints/zombie_anim.is_attacking` true _aszombie_anim)
        (set `CharacterMovementComponent.MaxWalkSpeed` 0.0 _charactermovement)
        (`KismetSystemLibrary.Delay` 0.5)
        (if _returnvalue
          (set `/Game/Blueprints/mecha_char+cam.TakingDamage` true _asmecha_char_cam))
        (`KismetSystemLibrary.Delay` 0.7)
        (set `/Game/Blueprints/zombie_anim.is_attacking` false _aszombie_anim)
        (set `CharacterMovementComponent.MaxWalkSpeed` 150.0 _charactermovement)))
    (:`OnSuccess`
      (goto _label))))

(event `self.ReceiveHit`
  (params (MyComp :type "PrimitiveComponent Object Reference") (Other :type "Actor Object Reference") (OtherComp :type "PrimitiveComponent Object Reference") (bSelfMoved :type Boolean) (HitLocation :type "Vector Structure") (HitNormal :type "Vector Structure") (NormalImpulse :type "Vector Structure") (Hit :type "HitResult Structure (by ref)"))
  (bind _mesh (`self.Mesh`))
  (bind _charactermovement (`self.CharacterMovement`))
  ;[1 1 1] take damage
  (bind _asbullet_actor (cast `/Game/trucs_a_nous/BulletActor` Other)
    (:`then`
      (bind _output_get (set `self.HP` (- (`self.HP`) 10)))
      (if (<= _output_get 0)
        (set `CharacterMovementComponent.MaxWalkSpeed` 0.0 _charactermovement)
        (`SkeletalMeshComponent.SetAllBodiesSimulatePhysics` _mesh true :!label _label_2)
        (`PrimitiveComponent.AddImpulseAtLocation` _mesh (* (`.ImpactNormal` (`GameplayStatics.BreakHitResult` Hit)) 30000.0) (`self.K2_GetActorLocation` _asbullet_actor) "None")
        (`ActorComponent.K2_DestroyComponent` (`self.CapsuleComponent`))
        (set `self.ided` true)
        (`KismetSystemLibrary.Delay` 30.0)
        (`self.K2_DestroyActor`)
        (else
          (set `CharacterMovementComponent.MaxWalkSpeed` 0.0 _charactermovement)
          (bind _aszombie_anim (cast `/Game/Blueprints/zombie_anim` (`SkeletalMeshComponent.GetAnimInstance` (`self.Mesh`))))
          (set `/Game/Blueprints/zombie_anim.take_damage` true _aszombie_anim)
          (`KismetSystemLibrary.Delay` 0.5)
          (set `/Game/Blueprints/zombie_anim.take_damage` false _aszombie_anim)
          (set `CharacterMovementComponent.MaxWalkSpeed` 150.0 _charactermovement))))
    (:`CastFailed`
      (cast `/Game/trucs_a_nous/marque_explosion` Other)
      (goto _label_2))))

(fn `UserConstructionScript`)